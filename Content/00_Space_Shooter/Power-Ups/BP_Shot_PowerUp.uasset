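; Shot power-up pickup for the space shooter that drifts along its forward vector every Tick at a set speed.
; On overlap with BP_SS_Character, it passes the power-up duration to ShotPowerUpPicked, attaches particle emitters to three fire points and plays a pickup sound.
; It removes its capsule and sphere but stays alive through a Delay of that duration, then destroys the emitters and itself.
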(event EventBeginPlay)

(event Collision|EventActorBeginOverlap
  (params (OtherActor :type Actor%20Object%20Reference))
  (bind _aspawn (Utilities|Casting|CastToPawn OtherActor))
  (bind _asbp_ss_character (Utilities|Casting|CastToBP_SS_Character _aspawn))
  (Default|ShotPowerUpPicked _asbp_ss_character (Variables|Default|GetShotPowerUpDuration))
  (bind (_emitter1 _emitter2 _emitter3) (CallFunction|SpawnEmitters (Variables|/Game/00_Space_Shooter/Players/BP_SS_Character.BP_SS_Character_C|GetFirePoint1 _asbp_ss_character) (Variables|/Game/00_Space_Shooter/Players/BP_SS_Character.BP_SS_Character_C|GetFirePoint2 _asbp_ss_character) (Variables|/Game/00_Space_Shooter/Players/BP_SS_Character.BP_SS_Character_C|GetFirePoint3 _asbp_ss_character)))
  (Audio|PlaySound2D "/Engine/VREditor/Sounds/UI/Dockable_Window_Pick_Up.Dockable_Window_Pick_Up" 1.0 1.0 0.0 0 0)
  (Components|DestroyComponent (Variables|Default|GetCapsule))
  (Components|DestroyComponent (Variables|Default|GetSphere))
  (Utilities|FlowControl|Delay (Variables|Default|GetShotPowerUpDuration))
  (Components|DestroyComponent _emitter1)
  (Components|DestroyComponent _emitter2)
  (Components|DestroyComponent _emitter3)
  (Actor|DestroyActor))

(event EventTick
  (params (DeltaSeconds :type Float%20%28single-precision%29))
  (Transformation|SetActorLocation (+ (Transformation|GetActorLocation) (* (Transformation|GetActorForwardVector) (* DeltaSeconds (Variables|Default|GetSpeed)))) false false))

(fn ConstructionScript)

(fn SpawnEmitters
  (params (FirePoint1 :type Scene%20Component%20Object%20Reference) (FirePoint2 :type Scene%20Component%20Object%20Reference) (FirePoint3 :type Scene%20Component%20Object%20Reference))
  (bind _returnvalue (Effects|SpawnEmitterAttached "/Game/00_Space_Shooter/Power-Ups/P_ShotPowerUp.P_ShotPowerUp" FirePoint1 "None"))
  (bind _returnvalue_2 (Effects|SpawnEmitterAttached "/Game/00_Space_Shooter/Power-Ups/P_ShotPowerUp.P_ShotPowerUp" FirePoint2 "None"))
  (bind _returnvalue_3 (Effects|SpawnEmitterAttached "/Game/00_Space_Shooter/Power-Ups/P_ShotPowerUp.P_ShotPowerUp" FirePoint3 "None"))
  (return _returnvalue _returnvalue_2 _returnvalue_3))