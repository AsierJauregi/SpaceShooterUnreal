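; BP_Healing_PowerUp is a space shooter pickup that heals the player character.
; Each tick it moves along its forward vector at its Speed value, without sweeping.
; On overlap with a BP_SS_Character pawn it calls HealActor on that character, plays a 2D sound and destroys itself.
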(event EventBeginPlay)

(event EventTick
  (params (DeltaSeconds :type Float%20%28single-precision%29))
  (Transformation|SetActorLocation (+ (Transformation|GetActorLocation) (* (Transformation|GetActorForwardVector) (* DeltaSeconds (Variables|Default|GetSpeed)))) false false))

(event Collision|EventActorBeginOverlap
  (params (OtherActor :type Actor%20Object%20Reference))
  (bind _aspawn (Utilities|Casting|CastToPawn OtherActor))
  (bind _asbp_ss_character (Utilities|Casting|CastToBP_SS_Character _aspawn))
  (Default|HealActor _asbp_ss_character)
  (Audio|PlaySound2D "/Engine/VREditor/Sounds/VR_open_Cue.VR_open_Cue" 1.0 1.0 0.0 0 0)
  (Actor|DestroyActor))

(fn ConstructionScript)