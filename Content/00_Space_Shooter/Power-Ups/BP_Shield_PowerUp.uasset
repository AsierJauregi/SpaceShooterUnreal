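; Shield power-up pickup for the space shooter that moves along its forward vector every tick at a set speed.
; Overlapping the tagged player character calls ActivateShield with the power-up duration and destroys the pickup.
; Touching an actor tagged BottomBorder also destroys it.
; A SpawnEmitters helper attaches shot power-up particles to three given fire points, but nothing in this Blueprint calls it.
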(event EventBeginPlay)

(event Collision|EventActorBeginOverlap
  (params (OtherActor :type Actor%20Object%20Reference))
  (if (Utilities|Array|ContainsItem (Variables|/Script/Engine.Actor|GetTags OtherActor) "Player")
    (bind _aspawn (Utilities|Casting|CastToPawn OtherActor))
    (bind _asbp_ss_character (Utilities|Casting|CastToBP_SS_Character _aspawn))
    (Default|ActivateShield _asbp_ss_character (Variables|Default|GetShieldPowerUpDuration))
    (Actor|DestroyActor)
    (elif (Utilities|Array|ContainsItem (Variables|/Script/Engine.Actor|GetTags OtherActor) "BottomBorder")
      (Actor|DestroyActor))))

(event EventTick
  (params (DeltaSeconds :type Float%20%28single-precision%29))
  (Transformation|SetActorLocation (+ (Transformation|GetActorLocation) (* (Transformation|GetActorForwardVector) (* DeltaSeconds (Variables|Default|GetSpeed)))) false false))

(fn ConstructionScript)

(fn SpawnEmitters
  (params (FirePoint1 :type Scene%20Component%20Object%20Reference) (FirePoint2 :type Scene%20Component%20Object%20Reference) (FirePoint3 :type Scene%20Component%20Object%20Reference))
  (bind _returnvalue (Effects|SpawnEmitterAttached "/Game/00_Space_Shooter/Power-Ups/P_ShotPowerUp.P_ShotPowerUp" FirePoint1 "None"))
  (bind _returnvalue_2 (Effects|SpawnEmitterAttached "/Game/00_Space_Shooter/Power-Ups/P_ShotPowerUp.P_ShotPowerUp" FirePoint2 "None"))
  (bind _returnvalue_3 (Effects|SpawnEmitterAttached "/Game/00_Space_Shooter/Power-Ups/P_ShotPowerUp.P_ShotPowerUp" FirePoint3 "None"))
  (return _returnvalue _returnvalue_2 _returnvalue_3))