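; Base enemy actor for the space shooter that flies straight along its initial forward vector and fires periodically.
; Tick moves it without sweep and accumulates time against a cooldown to spawn a shot at FirePoint, aligned to the enemy's rotation.
; Overlapping a Player-tagged actor fires the OnEnemyDestroy dispatcher, which destroys the enemy after a brief delay, and notifies BP_SS_Gamemode.
; A BP_Projectile cast in the graph is disconnected.
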(event Custom|Destroyed_Event
  (Utilities|FlowControl|Delay 0.1)
  (Actor|DestroyActor))

(event EventBeginPlay
  (Variables|Default|SetMovementVector (Transformation|GetActorForwardVector))
  (EventDispatchers|BindEventtoOnEnemyDestroy (delegate Custom|Destroyed_Event)))

(event Collision|EventActorBeginOverlap
  (params (OtherActor :type Actor%20Object%20Reference))
  (if (Utilities|Array|ContainsItem (Variables|/Script/Engine.Actor|GetTags OtherActor) "Player")
    (Default|CallOnEnemyDestroy)
    (bind _asbp_ss_gamemode (Utilities|Casting|CastToBP_SS_Gamemode (Game|GetGameMode)))
    (Default|EnemyDestroyed _asbp_ss_gamemode)))

(event EventTick
  (params (DeltaSeconds :type Float%20%28single-precision%29))
  (CallFunction|Move DeltaSeconds)
  (bind _output_get (Variables|Default|SetShotCurrentTime (+ DeltaSeconds (Variables|Default|GetShotCurrentTime))))
  (if (< (Variables|Default|GetShotCooldown) _output_get)
    (Variables|Default|SetShotCurrentTime 0.0)
    (CallFunction|Shoot)))

(fn ConstructionScript)

(fn Move
  (params (Delta%20Time :type Float%20%28double-precision%29))
  (Transformation|SetActorLocation (+ (Transformation|GetActorLocation) (* (* Delta%20Time (Variables|Default|GetSpeed)) (Variables|Default|GetMovementVector))) false false))

(fn Shoot
  (bind _returnvalue (Game|SpawnActorfromClass (Variables|Default|GetClass) (Transformation|GetWorldTransform (Variables|Default|GetFirePoint)) "Undefined" "MultiplyWithRoot" 0 0))
  (Transformation|SetActorRotation _returnvalue (Transformation|GetActorRotation)))